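; AI controller for guard NPCs that runs BT_GuardAI_OV to fight sensed actors not tagged "Enemy".
; Perception writes a sensed target to the Enemy blackboard key after a short random reaction delay; other updates clear it after a fixed delay.
; Tick sets the pawn's Aiming and Shooting flags whenever a focus actor exists.
; The LastSeenLocation blackboard write is unconnected and never runs.
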(event OnTargetPerceptionUpdated(AIPerception)
  (params (Actor :type Actor%20Object%20Reference) (Stimulus :type AI%20Stimulus%20Structure))
  (if (and (not (Actor|ActorHasTag Actor "Enemy")) (.bsuccessfullysensed Stimulus))
    (Utilities|FlowControl|Delay (Math|Random|RandomFloatinRange 0.0 0.4))
    (AI|Components|Blackboard|SetValueasObject (AI|GetBlackboard 0) (Variables|Default|GetEnemy) Actor)
    (else
      (Utilities|FlowControl|Delay 1.0)
      (AI|Components|Blackboard|ClearValue (AI|GetBlackboard 0) (Variables|Default|GetEnemy)))))

(event EventBeginPlay
  (AI|RunBehaviorTree "/Game/Dynamic/NPC/AI/BT_GuardAI_OV.BT_GuardAI_OV"))

(event EventTick
  (params (DeltaSeconds :type Float%20%28single-precision%29))
  (bind _returnvalue (Class|AIController|GetFocusActor))
  (bind _returnvalue_2 (Utilities|IsValid _returnvalue))
  (bind _astpcharacter (Utilities|Casting|CastToTPCharacter (Pawn|GetControlledPawn)))
  (Variables|/Game/Dynamic/NPC/Blueprints/TPCharacter.TPCharacter_C|SetAiming _astpcharacter _returnvalue_2)
  (Variables|/Game/Dynamic/NPC/Blueprints/TPCharacter.TPCharacter_C|SetShooting _astpcharacter _returnvalue_2))

(fn ConstructionScript)