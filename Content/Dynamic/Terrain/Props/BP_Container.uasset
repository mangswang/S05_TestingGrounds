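; BP_Container is a shipping-container prop that randomizes its door layout and color for visual variety.
; The construction script gives each door a random yaw and, a quarter of the time, destroys a door, always DoorR because RandomInteger(1) only returns 0.
; BeginPlay turns a random unit vector into a color and applies it through dynamic material instances to the body and any surviving doors.
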(event EventBeginPlay
  (bind _doorl (Variables|Default|GetDoorL))
  (bind _doorr (Variables|Default|GetDoorR))
  (Variables|Default|SetColour (Math|Conversions|ToLinearColor(Vector) (Math|Random|RandomUnitVector)))
  (Utilities|FlowControl|Sequence
    (:then_0
      (bind _returnvalue (Rendering|Material|CreateDynamicMaterialInstance (Variables|Default|GetContainer) 0 0 "None" :!class /Script/Engine.PrimitiveComponent))
      (Rendering|Material|SetVectorParameterValue _returnvalue "diffuse color" (Variables|Default|GetColour) :!class /Script/Engine.MaterialInstanceDynamic))
    (:then_1
      (Utilities|IsValid _doorl
        (:Is%20Valid
          (bind _returnvalue_2 (Rendering|Material|CreateDynamicMaterialInstance _doorl 0 0 "None" :!class /Script/Engine.PrimitiveComponent))
          (Rendering|Material|SetVectorParameterValue _returnvalue_2 "diffuse color" (Variables|Default|GetColour) :!class /Script/Engine.MaterialInstanceDynamic))))
    (:then_2
      (Utilities|IsValid _doorr
        (:Is%20Valid
          (bind _returnvalue_3 (Rendering|Material|CreateDynamicMaterialInstance _doorr 0 0 "None" :!class /Script/Engine.PrimitiveComponent))
          (Rendering|Material|SetVectorParameterValue _returnvalue_3 "diffuse color" (Variables|Default|GetColour) :!class /Script/Engine.MaterialInstanceDynamic))))))

(event Collision|EventActorBeginOverlap
  (params (OtherActor :type Actor%20Object%20Reference)))

(event EventTick
  (params (DeltaSeconds :type Float%20%28single-precision%29)))

(fn ConstructionScript
  (Transformation|SetRelativeRotation (Variables|Default|GetDoorR) (Math|Rotator|MakeRotator 0.0 0.0 (Math|Conversions|ToFloat(Integer) (Math|Random|RandomIntegerinRange (Math|Integer|SelectInt 0 -70 (> (Math|Random|RandomFloatinRange 0.0 1.0) 0.5)) -120))) false false)
  (Transformation|SetRelativeRotation (Variables|Default|GetDoorL) (Math|Rotator|MakeRotator 0.0 0.0 (Math|Conversions|ToFloat(Integer) (Math|Random|RandomIntegerinRange (Math|Integer|SelectInt 0 70 (> (Math|Random|RandomFloatinRange 0.0 1.0) 0.5)) 120))) false false)
  (if (not (> (Math|Random|RandomFloatinRange 0.0 1.0) 0.25))
    (Components|DestroyComponent (Utilities|Select :Index (Math|Random|RandomInteger 1) :Option%200 (Variables|Default|GetDoorR) :Option%201 (Variables|Default|GetDoorL)))))