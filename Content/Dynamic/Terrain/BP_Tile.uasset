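; BP_Tile is one segment of an infinite terrain, dressed with randomly placed props and AI characters whose count grows with the tile number.
; A gate starts locked, opens while the player overlaps LockingVolume, then relocks on exit and reports the tile conquered once to InfiniteTerrainGM.
; When the player reaches DestroyVolume, it asks the game mode to spawn another tile and destroys itself.
; An arrow provides the attach transform.
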(event OnComponentEndOverlap(LockingVolume)
  (params (OverlappedComponent :type Primitive%20Component%20Object%20Reference) (OtherActor :type Actor%20Object%20Reference) (OtherComp :type Primitive%20Component%20Object%20Reference) (OtherBodyIndex :type Integer))
  (Utilities|IsPlayerChar? OtherActor)
  (CallFunction|Lock)
  (Utilities|FlowControl|DoOnce false
    (:Completed
      (Default|NewTileConquered (Variables|Default|GetGMRef)))))

(event OnComponentBeginOverlap(LockingVolume)
  (params (OverlappedComponent :type Primitive%20Component%20Object%20Reference) (OtherActor :type Actor%20Object%20Reference) (OtherComp :type Primitive%20Component%20Object%20Reference) (OtherBodyIndex :type Integer) (bFromSweep :type Boolean) (SweepResult :type Hit%20Result%20Structure%20%28by%20ref%29))
  (Utilities|IsPlayerChar? OtherActor)
  (CallFunction|Unlock))

(event OnComponentBeginOverlap(DestroyVolume)
  (params (OverlappedComponent :type Primitive%20Component%20Object%20Reference) (OtherActor :type Actor%20Object%20Reference) (OtherComp :type Primitive%20Component%20Object%20Reference) (OtherBodyIndex :type Integer) (bFromSweep :type Boolean) (SweepResult :type Hit%20Result%20Structure%20%28by%20ref%29))
  (Utilities|IsPlayerChar? OtherActor)
  (Default|SpawnTile (Variables|Default|GetGMRef))
  (Actor|DestroyActor))

(event EventBeginPlay
  (bind _asinfinite_terrain_gm (Utilities|Casting|CastToInfiniteTerrainGM (Game|GetGameMode)))
  (Variables|Default|SetGMRef _asinfinite_terrain_gm)
  (CallFunction|Lock)
  (Variables|Default|SetLocalTileNumber (Variables|/Game/Dynamic/InfiniteTerrainGM.InfiniteTerrainGM_C|GetTileNumber _asinfinite_terrain_gm))
  (Utilities|FlowControl|Sequence
    (:then_0
      (CallFunction|SpawnActors))
    (:then_1
      (if (> (Variables|Default|GetLocalTileNumber) 1)
        (if (>= (Variables|Default|GetLocalTileNumber) 100)
          (Class|Tile|PlaceAIPawns "/Game/Dynamic/Character/Blueprints/BP_Character.BP_Character_C" 10 50 2e+02)
          (else
            (Class|Tile|PlaceAIPawns "/Game/Dynamic/Character/Blueprints/BP_Character.BP_Character_C" 1 (Math|Integer|Clamp(Integer) (/ (Variables|Default|GetLocalTileNumber) 3) 1 10) 2e+02)))))))

(fn ConstructionScript)

(fn GetAttachLocation
  (return (Transformation|GetWorldTransform (Variables|Default|GetArrow))))

(fn Unlock
  (bind _gate (Variables|Default|GetGate))
  (Collision|SetCollisionEnabled _gate "NoCollision")
  (Rendering|Material|SetMaterial _gate 0 "/Game/Dynamic/Terrain/MI_Barrier_Green.MI_Barrier_Green"))

(fn Lock
  (bind _gate (Variables|Default|GetGate))
  (Collision|SetCollisionEnabled _gate "QueryAndPhysics")
  (Rendering|Material|SetMaterial _gate 0 "/Game/Dynamic/Terrain/MI_Barrier_Red.MI_Barrier_Red"))

(fn SpawnActors
  (Class|Tile|PlaceActors "/Game/Dynamic/Terrain/Props/BP_Container.BP_Container_C" 0 3 7e+02 1.0 1.0)
  (Class|Tile|PlaceActors "/Game/Dynamic/Terrain/Props/BP_SandBags.BP_SandBags_C" 0 5 4.5e+02 1.0 1.0)
  (Class|Tile|PlaceActors "/Game/Dynamic/Terrain/Props/BP_Rock3.BP_Rock3_C" 0 5 4.5e+02 0.1 3.0)
  (Class|Tile|PlaceActors "/Game/Dynamic/Terrain/Props/BP_Rock2.BP_Rock2_C" 0 5 4e+02 0.1 3.0)
  (Class|Tile|PlaceActors "/Game/Dynamic/Terrain/Props/BP_Rock1.BP_Rock1_C" 0 10 1.5e+02 0.1 3.0)
  (Class|Tile|PlaceActors "/Game/Dynamic/Terrain/Props/BP_Box.BP_Box_C" 0 5 1e+02 0.5 2.0)
  (Class|Tile|PlaceActors "/Game/Dynamic/Terrain/Props/BP_Canister.BP_Canister_C" 0 5 5e+01 0.5 1.2))