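; Terrain tile Blueprint for an endless terrain, with a gate and an arrow marking an attach transform.
; The gate starts locked, toggling collision and red/green barrier materials to open while the player overlaps the locking volume.
; When the player leaves that volume, the gate relocks and the InfiniteTerrainGM game mode spawns a tile.
; The tile destroys itself when the player enters its destroy volume.
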(event OnComponentEndOverlap(LockingVolume)
  (params (OverlappedComponent :type Primitive%20Component%20Object%20Reference) (OtherActor :type Actor%20Object%20Reference) (OtherComp :type Primitive%20Component%20Object%20Reference) (OtherBodyIndex :type Integer))
  (Utilities|IsPlayerChar? OtherActor)
  (CallFunction|Lock)
  (Default|SpawnTile (Variables|Default|GetGMRef)))

(event OnComponentBeginOverlap(LockingVolume)
  (params (OverlappedComponent :type Primitive%20Component%20Object%20Reference) (OtherActor :type Actor%20Object%20Reference) (OtherComp :type Primitive%20Component%20Object%20Reference) (OtherBodyIndex :type Integer) (bFromSweep :type Boolean) (SweepResult :type Hit%20Result%20Structure%20%28by%20ref%29))
  (Utilities|IsPlayerChar? OtherActor)
  (CallFunction|Unlock))

(event OnComponentBeginOverlap(DestroyVolume)
  (params (OverlappedComponent :type Primitive%20Component%20Object%20Reference) (OtherActor :type Actor%20Object%20Reference) (OtherComp :type Primitive%20Component%20Object%20Reference) (OtherBodyIndex :type Integer) (bFromSweep :type Boolean) (SweepResult :type Hit%20Result%20Structure%20%28by%20ref%29))
  (Utilities|IsPlayerChar? OtherActor)
  (Actor|DestroyActor))

(event EventBeginPlay
  (bind _asinfinite_terrain_gm (Utilities|Casting|CastToInfiniteTerrainGM (Game|GetGameMode)))
  (Variables|Default|SetGMRef _asinfinite_terrain_gm)
  (CallFunction|Lock))

(fn ConstructionScript)

(fn GetAttachLocation
  (return (Transformation|GetWorldTransform (Variables|Default|GetArrow))))

(fn Unlock
  (bind _gate (Variables|Default|GetGate))
  (Collision|SetCollisionEnabled _gate "NoCollision")
  (Rendering|Material|SetMaterial _gate 0 "/Game/Dynamic/Terrain/GreenBarrier.GreenBarrier"))

(fn Lock
  (bind _gate (Variables|Default|GetGate))
  (Collision|SetCollisionEnabled _gate "QueryAndPhysics")
  (Rendering|Material|SetMaterial _gate 0 "/Game/Dynamic/Terrain/RedBarrier.RedBarrier"))